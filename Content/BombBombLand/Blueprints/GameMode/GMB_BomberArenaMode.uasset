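; Game mode for the Bomber arena that builds the level, spawns local players and runs a match countdown.
; At BeginPlay it thins placed crates by randomly destroying a DeletePercentage share of them.
; It then spawns and possesses a BP_Player at each PlayerStart, creating local players and adding the input mapping context.
; Tick uses a one-second Delay to count down Minutes and Seconds, printing Game Over at zero.
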(event `self.ReceiveBeginPlay`
  (`self.GenerateLevel`)
  (bind _outactors (`GameplayStatics.GetAllActorsOfClass` "/Script/Engine.PlayerStart"))
  (for (_array_element _array_index) _outactors
    (bind _output_get (set `self.Array Index` _array_index))
    (bind _returnvalue (`GameplayStatics.CreatePlayer` _output_get))
    (if (> (`self.Array Index`) 0)
      (`EnhancedInputSubsystemInterface.AddMappingContext` (pcsubsystem `EnhancedInputLocalPlayerSubsystem` _returnvalue) "/Game/BombBombLand/Blueprints/Input/IMC_PlayerControls.IMC_PlayerControls" 0 (struct))
      (bind _returnvalue_2 (`self.GetTransform` _array_element))
      (bind _returnvalue_3 (`|SpawnActorFromClass` "/Game/BombBombLand/Blueprints/Character/BP_Player.BP_Player_C" _returnvalue_2 "Undefined" "MultiplyWithRoot" null null))
      (`Controller.Possess` (`GameplayStatics.GetPlayerController` (`self.Array Index`)) _returnvalue_3)
      (else
        (`EnhancedInputSubsystemInterface.AddMappingContext` (pcsubsystem `EnhancedInputLocalPlayerSubsystem` (`GameplayStatics.GetPlayerController` 0)) "/Game/BombBombLand/Blueprints/Input/IMC_PlayerControls.IMC_PlayerControls" 0 (struct))
        (bind _returnvalue_4 (`|SpawnActorFromClass` "/Game/BombBombLand/Blueprints/Character/BP_Player.BP_Player_C" _returnvalue_2 "Undefined" "MultiplyWithRoot" null null))
        (`Controller.Possess` (`GameplayStatics.GetPlayerController` 0) _returnvalue_4)))))

(event `self.ReceiveTick`
  (params (DeltaSeconds :type "Float (single-precision)"))
  (`KismetSystemLibrary.Delay` 1.0)
  (if (== (`self.Seconds`) 0)
    (if (== (`self.Minutes`) 0)
      (`KismetSystemLibrary.PrintString` "Game Over")
      (else
        (set `self.Seconds` 59)
        (set `self.Minutes` (- (`self.Minutes`) 1))))
    (else
      (set `self.Seconds` (- (`self.Seconds`) 1)))))

(fn `GenerateLevel`
  (bind _outactors (`GameplayStatics.GetAllActorsOfClass` "/Game/BombBombLand/Blueprints/Items/BP_Crates.BP_Crates_C"))
  (set `self.Crates` _outactors)
  (for _ (range (+ (`KismetMathLibrary.FTrunc` (* (`KismetArrayLibrary.Array_Length` _outactors) (`self.DeletePercentage`))) 1))
    (bind _output_get (set `self.RandomCrate` (`KismetArrayLibrary.Array_Random` (`self.Crates`))))
    (`self.K2_DestroyActor` _output_get)
    (`KismetArrayLibrary.Array_RemoveItem` (`self.Crates`) (`self.RandomCrate`)))
  (set `self.GameSetup` false))

(fn `UserConstructionScript`)