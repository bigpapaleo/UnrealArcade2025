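; BP_Teleport is a trigger in BombBombLand that moves a BP_BombBombCharacter to the position of its Location actor.
; Overlapping its Box starts a white camera fade on player 0, then after a delay moves the character without sweep.
; The capsule ignores WorldDynamic collision from just before the move until a second delay ends, then blocks it again.
; A second fade with the same to-white settings starts right after the move.
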(event `self.ReceiveBeginPlay`)

(event `self.Box.OnComponentBeginOverlap`
  (params (OverlappedComponent :type "PrimitiveComponent Object Reference") (OtherActor :type "Actor Object Reference") (OtherComp :type "PrimitiveComponent Object Reference") (OtherBodyIndex :type Integer) (bFromSweep :type Boolean) (SweepResult :type "HitResult Structure (by ref)"))
  (bind _returnvalue (`GameplayStatics.GetPlayerCameraManager` 0))
  (bind _asbp_bomb_bomb_character (cast `/Game/BombBombLand/ThirdPerson/Blueprints/BP_BombBombCharacter` OtherActor))
  (`PlayerCameraManager.StartCameraFade` _returnvalue 0.0 1.0 1.0 (struct :`R` 1.0 :`G` 1.0 :`B` 1.0 :`A` 1.0) false false)
  (`KismetSystemLibrary.Delay` 1.5)
  (bind _capsulecomponent (`Character.CapsuleComponent` _asbp_bomb_bomb_character))
  (`PrimitiveComponent.SetCollisionResponseToChannel` _capsulecomponent "ECC_WorldDynamic" "ECR_Ignore")
  (`self.K2_SetActorLocation` _asbp_bomb_bomb_character (`self.K2_GetActorLocation` (`self.Location`)) false false)
  (`PlayerCameraManager.StartCameraFade` _returnvalue 0.0 1.0 1.0 (struct :`R` 1.0 :`G` 1.0 :`B` 1.0 :`A` 1.0) false false)
  (`KismetSystemLibrary.Delay` 3.0)
  (`PrimitiveComponent.SetCollisionResponseToChannel` _capsulecomponent "ECC_WorldDynamic" "ECR_Block"))

(fn `UserConstructionScript`)