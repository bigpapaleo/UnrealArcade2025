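; BP_Player is the Bomberman-style player character, moved along world axes by Enhanced Input and able to plant bombs.
; SC_PlantBomb spawns grid-snapped BP_Bombs up to BombCount, passing BombStrength and untracking each on EndPlay.
; OP_ClearBombCollision toggles capsule move-ignore, and each bomb's leave-collision event clears it.
; Clamped upgrade and downgrade events adjust bomb count, strength and walk speed, though DowngradeSpeed divides by 50 where UpgradeSpeed multiplies.
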(event `self.ReceiveBeginPlay`
  (`EnhancedInputSubsystemInterface.AddMappingContext` (pcsubsystem `EnhancedInputLocalPlayerSubsystem` (`GameplayStatics.GetPlayerController` 0)) "/Game/BombBombLand/Blueprints/Input/IMC_PlayerControls.IMC_PlayerControls" 0 (struct)))

(event `OP_ClearBombCollision`
  (params (BombHasCollision :type Boolean) (PrimitiveComponent :type "PrimitiveComponent Object Reference"))
  (if BombHasCollision
    (`PrimitiveComponent.ClearMoveIgnoreComponents` (`self.CapsuleComponent`))
    (else
      (`PrimitiveComponent.IgnoreComponentWhenMoving` (`self.CapsuleComponent`) PrimitiveComponent true))))

(event `EnhancedInput|/Game/BombBombLand/Blueprints/Input/IA_Movement`
  (params (ActionValue :type "Vector2D Structure") (ElapsedSeconds :type "Float (double-precision)") (TriggeredSeconds :type "Float (double-precision)") (InputAction :type "InputAction Object Reference" :default "/Game/BombBombLand/Blueprints/Input/IA_Movement.IA_Movement"))
  (:`Triggered`
    (`self.AddMovementInput` (0.0 1.0 0.0) ActionValue_X)
    (`self.AddMovementInput` (1.0 0.0 0.0) ActionValue_Y)))

(event `SC_PlantBomb`
  (bind _returnvalue (`self.K2_GetActorLocation`))
  (bind (_returnvalue_x _returnvalue_y _returnvalue_z) (`KismetMathLibrary.BreakVector` (`KismetMathLibrary.Vector_SnappedToGrid` _returnvalue 200.0)))
  (bind (_returnvalue_x_2 _returnvalue_y_2) (`KismetMathLibrary.BreakVector` (`KismetMathLibrary.Vector_SnappedToGrid` _returnvalue 100.0)))
  (if (< (`KismetArrayLibrary.Array_Length` (`self.PlacedBombs`)) (`self.BombCount`))
    (bind _returnvalue_2 (`|SpawnActorFromClass` "/Game/BombBombLand/Blueprints/Items/BP_Bomb.BP_Bomb_C" (`KismetMathLibrary.MakeTransform` (`KismetMathLibrary.MakeVector` _returnvalue_x_2 _returnvalue_y_2 _returnvalue_z)) "AlwaysSpawn" "MultiplyWithRoot" self (`self.Bomb Strength`) null))
    (`KismetArrayLibrary.Array_AddUnique` (`self.PlacedBombs`) _returnvalue_2)
    (add `/Game/BombBombLand/Blueprints/Items/BP_Bomb.LeaveBombCollision` _returnvalue_2 (delegate `ClearbombCollision`))
    (add `self.OnEndPlay` _returnvalue_2 (delegate `OnBombDestroyed`))))

(event `ClearbombCollision`
  (`self.OP_ClearBombCollision` true))

(event `OnBombDestroyed` :!signature `self.OnEndPlay`
  (params (Actor :type "Actor Object Reference") (EndPlayReason :type "EEndPlayReason Enum" :default "Destroyed"))
  (`KismetArrayLibrary.Array_RemoveItem` (`self.PlacedBombs`) Actor))

(event `EnhancedInput|/Game/BombBombLand/Blueprints/Input/IA_Bomb`
  (params (ActionValue :type Boolean) (ElapsedSeconds :type "Float (double-precision)") (TriggeredSeconds :type "Float (double-precision)") (InputAction :type "InputAction Object Reference" :default "/Game/BombBombLand/Blueprints/Input/IA_Bomb.IA_Bomb"))
  (:`Started`
    (`self.SC_PlantBomb`)))

(event `UpgradeSpeed`
  (bind _output_get (set `self.SpeedUpgrade` (`KismetMathLibrary.Clamp` (+ (`self.SpeedUpgrade`) 1) 0 10)))
  (set `CharacterMovementComponent.MaxWalkSpeed` (+ (* _output_get 50) 400.0) (`self.CharacterMovement`)))

(event `UpgradeBombStrength`
  (set `self.Bomb Strength` (`KismetMathLibrary.Clamp` (+ (`self.Bomb Strength`) 1) 0 10)))

(event `UpgradeBombCount`
  (set `self.BombCount` (`KismetMathLibrary.Clamp` (+ (`self.BombCount`) 1) 0 10)))

(event `DowngradeBombs`
  (set `self.BombCount` (`KismetMathLibrary.Clamp` (- (`self.BombCount`) 1) 1 10)))

(event `DowngradeFirePow`
  (set `self.Bomb Strength` (`KismetMathLibrary.Clamp` (- (`self.Bomb Strength`) 1) 1 10)))

(event `DowngradeSpeed`
  (bind _output_get (set `self.SpeedUpgrade` (`KismetMathLibrary.Clamp` (- (`self.SpeedUpgrade`) 1) 1 10)))
  (set `CharacterMovementComponent.MaxWalkSpeed` (+ (/ _output_get 50) 400.0) (`self.CharacterMovement`)))

(fn `UserConstructionScript`)