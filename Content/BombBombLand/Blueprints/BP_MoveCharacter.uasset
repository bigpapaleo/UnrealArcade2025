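; BP_MoveCharacter is a trigger volume in BombBombLand that automatically walks the player character to a goal actor.
; When a BP_BombBombCharacter overlaps its Box, it disables input, starts SimpleMoveToActor toward Goal and sets the capsule to ignore WorldDynamic collision.
; After a set Duration it re-enables input and restores blocking, on a fixed timer rather than an arrival check.
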(event `self.Box.OnComponentBeginOverlap`
  (params (OverlappedComponent :type "PrimitiveComponent Object Reference") (OtherActor :type "Actor Object Reference") (OtherComp :type "PrimitiveComponent Object Reference") (OtherBodyIndex :type Integer) (bFromSweep :type Boolean) (SweepResult :type "HitResult Structure (by ref)"))
  (bind _returnvalue (`GameplayStatics.GetPlayerController` 0))
  (bind _asbp_bomb_bomb_character (cast `/Game/BombBombLand/ThirdPerson/Blueprints/BP_BombBombCharacter` OtherActor))
  (`self.DisableInput` _asbp_bomb_bomb_character _returnvalue)
  (`AIBlueprintHelperLibrary.SimpleMoveToActor` _returnvalue (`self.Goal`))
  (bind _capsulecomponent (`Character.CapsuleComponent` _asbp_bomb_bomb_character))
  (`PrimitiveComponent.SetCollisionResponseToChannel` _capsulecomponent "ECC_WorldDynamic" "ECR_Ignore")
  (`KismetSystemLibrary.Delay` (`self.Duration`))
  (`self.EnableInput` _asbp_bomb_bomb_character _returnvalue)
  (`PrimitiveComponent.SetCollisionResponseToChannel` _capsulecomponent "ECC_WorldDynamic" "ECR_Block"))

(fn `UserConstructionScript`)