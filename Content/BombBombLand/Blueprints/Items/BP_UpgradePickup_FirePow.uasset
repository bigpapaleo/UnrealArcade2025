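; BP_UpgradePickup_FirePow is a pickup that upgrades the bomb strength of the player who touches it.
; On overlap, after calling the parent handler, only the authority casts the other actor to BP_Player and calls UpgradeBombStrength.
; It then plays the pickup sound in 2D on that authority instance and destroys itself.
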(event `self.ReceiveBeginPlay`
  (`parent.ReceiveBeginPlay`))

(event `self.ReceiveActorBeginOverlap`
  (params (OtherActor :type "Actor Object Reference"))
  (`parent.ReceiveActorBeginOverlap` OtherActor)
  (`/Engine/EditorBlueprintResources/ActorMacros.Switch Has Authority`
    (:`Authority`
      (bind _asbp_player (cast `/Game/BombBombLand/Blueprints/Character/BP_Player` OtherActor))
      (`/Game/BombBombLand/Blueprints/Character/BP_Player.UpgradeBombStrength` _asbp_player)
      (`GameplayStatics.PlaySound2D` "/Game/BombBombLand/Audio/Sounds/FX/PickupSound_Cue.PickupSound_Cue" 1.0 1.0 0.0 null null)
      (`self.K2_DestroyActor`))))

(fn `UserConstructionScript`
  (`parent.UserConstructionScript`))