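; Bomb actor owned by a BP_Player that counts down and explodes in four perpendicular directions.
; On spawn the owner's capsule ignores its blocking box, and any overlap end broadcasts LeaveBombCollision.
; A timeline scales the mesh and finishes with sound and shockwave effects, while an authority-only timer triggers Explode.
; Explode spawns explosion effects and four BP_ExplosionProjectiles carrying BombStrength, then destroys the bomb.
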(event `self.ReceiveActorEndOverlap`
  (params (OtherActor :type "Actor Object Reference"))
  (`self.LeaveBombCollision`))

(event `Explode`
  (bind _returnvalue (+ (`self.K2_GetActorLocation`) (0.0 0.0 5.0)))
  (`self.SetActorEnableCollision` false)
  (for _index (range 4)
    (`|SpawnActorFromClass` "/Game/BombBombLand/Blueprints/BP_ExplosionProjectile.BP_ExplosionProjectile_C" (`KismetMathLibrary.MakeTransform` _returnvalue (`KismetMathLibrary.Conv_VectorToRotator` (`KismetMathLibrary.GreaterGreater_VectorRotator` (1.0 0.0 0.0) (`KismetMathLibrary.MakeRotator` 0.0 0.0 (`KismetMathLibrary.Conv_IntToDouble` (* _index 90)))))) "Undefined" "MultiplyWithRoot" self (`self.BombStrength`) null)
    (`NiagaraFunctionLibrary.SpawnSystemAtLocation` "/Game/BombBombLand/Particles/P_Explosion.P_Explosion" _returnvalue))
  (`self.K2_DestroyActor`))

(event `self.ReceiveBeginPlay`
  (`PrimitiveComponent.IgnoreComponentWhenMoving` (`Character.CapsuleComponent` (cast `/Game/BombBombLand/Blueprints/Character/BP_Player` (`self.GetOwner`) :!pure true)) (`self.BlockBox`) true)
  (`|ExecutionSequence`
    (:`then_0`
      (bind (_direction _bombscale) (`Timeline|Exploding`)
        (:`Update`
          (`SceneComponent.SetWorldScale3D` (`self.SM_Bomb`) (`KismetMathLibrary.Conv_DoubleToVector` _bombscale)))
        (:`Finished`
          (`GameplayStatics.PlaySoundAtLocation` "/Game/BombBombLand/Audio/Sounds/FX/SC_BombExplosion.SC_BombExplosion" (`self.K2_GetActorLocation`) (struct) 1.0 1.0 0.0 null null null null)
          (`NiagaraFunctionLibrary.SpawnSystemAtLocation` "/Game/BombBombLand/Particles/P_SoundShock.P_SoundShock" (+ (`self.K2_GetActorLocation`) (0.0 0.0 100.0)) (struct) (1.0 1.0 1.0) true true "AutoRelease"))))
    (:`then_1`
      (`/Engine/EditorBlueprintResources/ActorMacros.Switch Has Authority`
        (:`Authority`
          (`KismetSystemLibrary.K2_SetTimerDelegate` (delegate `Explode`) 3.0))))))

(fn `UserConstructionScript`)