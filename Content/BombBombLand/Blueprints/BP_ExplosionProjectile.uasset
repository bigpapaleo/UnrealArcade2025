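; Explosion projectile for bomb blasts, with a lifespan scaled by BombStrength that limits how long the blast lasts.
; Sphere overlaps detonate other bombs without stopping the projectile, while hit characters receive a bombed event and "Bombable"-tagged actors get a short lifespan, both ending the projectile.
; Any blocking hit also destroys it; the sphere ignores its owner when moving, and debug prints name what it touches.
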(event `self.ReceiveBeginPlay`
  (`self.SetLifeSpan` (* (`self.BombStrength`) 0.1))
  (`NiagaraComponent.SetAutoDestroy` (`self.Niagara`) false)
  (`PrimitiveComponent.IgnoreActorWhenMoving` (`self.Sphere1`) (`self.GetOwner`) true))

(event `self.Sphere1.OnComponentBeginOverlap`
  (params (OverlappedComponent :type "PrimitiveComponent Object Reference") (OtherActor :type "Actor Object Reference") (OtherComp :type "PrimitiveComponent Object Reference") (OtherBodyIndex :type Integer) (bFromSweep :type Boolean) (SweepResult :type "HitResult Structure (by ref)"))
  (`KismetSystemLibrary.PrintString` (`KismetSystemLibrary.GetDisplayName` OtherActor))
  (bind _asbp_bomb (cast `/Game/BombBombLand/Blueprints/Items/BP_Bomb` OtherActor)
    (:`then`
      (`/Game/BombBombLand/Blueprints/Items/BP_Bomb.Explode` _asbp_bomb))
    (:`CastFailed`
      (bind _asbp_bomb_bomb_character (cast `/Game/BombBombLand/ThirdPerson/Blueprints/BP_BombBombCharacter` OtherActor)
        (:`then`
          (`/Game/BombBombLand/ThirdPerson/Blueprints/BP_BombBombCharacter.Event_Bombed` _asbp_bomb_bomb_character)
          (`self.K2_DestroyActor` :!label _label))
        (:`CastFailed`
          (if (`self.ActorHasTag` OtherActor "Bombable")
            (`self.SetLifeSpan` OtherActor 0.1)
            (goto _label)))))))

(event `self.ReceiveHit`
  (params (MyComp :type "PrimitiveComponent Object Reference") (Other :type "Actor Object Reference") (OtherComp :type "PrimitiveComponent Object Reference") (bSelfMoved :type Boolean) (HitLocation :type "Vector Structure") (HitNormal :type "Vector Structure") (NormalImpulse :type "Vector Structure") (Hit :type "HitResult Structure (by ref)"))
  (`KismetSystemLibrary.PrintString` (`KismetSystemLibrary.GetDisplayName` OtherComp))
  (`self.K2_DestroyActor`))

(fn `UserConstructionScript`)