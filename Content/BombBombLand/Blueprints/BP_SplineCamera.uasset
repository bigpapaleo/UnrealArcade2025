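; BP_SplineCamera is a rail camera that takes over the player's view while its sphere trigger is overlapped.
; Begin overlap, unfiltered by actor, blends the view to this actor; end overlap by BP_BombBombCharacter2 blends back to that character.
; Each tick moves the spring arm to the spline point nearest the player, using fixed downward pitch, spline-direction yaw and look-at roll.
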(event `self.Sphere.OnComponentBeginOverlap`
  (params (OverlappedComponent :type "PrimitiveComponent Object Reference") (OtherActor :type "Actor Object Reference") (OtherComp :type "PrimitiveComponent Object Reference") (OtherBodyIndex :type Integer) (bFromSweep :type Boolean) (SweepResult :type "HitResult Structure (by ref)"))
  (`PlayerController.SetViewTargetWithBlend` (`GameplayStatics.GetPlayerController` 0) self 2.0 "VTBlend_Linear" 0.0 false))

(event `self.ReceiveTick`
  (params (DeltaSeconds :type "Float (single-precision)"))
  (bind _returnvalue (`GameplayStatics.GetPlayerCharacter` 0))
  (bind _springarm (`self.SpringArm`))
  (bind _spline (`self.Spline`))
  (bind _returnvalue_2 (`self.K2_GetActorLocation` _returnvalue))
  (bind _returnvalue_roll (`KismetMathLibrary.BreakRotator` (`KismetMathLibrary.FindLookAtRotation` (`SceneComponent.K2_GetComponentLocation` (`self.CineCamera`)) (`self.K2_GetActorLocation` _returnvalue))))
  (bind (_returnvalue_roll_2 _returnvalue_pitch _returnvalue_yaw) (`KismetMathLibrary.BreakRotator` (`KismetMathLibrary.Conv_VectorToRotator` (`SplineComponent.FindDirectionClosestToWorldLocation` _spline _returnvalue_2 "World"))))
  (`SceneComponent.K2_SetWorldLocation` _springarm (`SplineComponent.FindLocationClosestToWorldLocation` _spline _returnvalue_2 "World") false false)
  (`SceneComponent.K2_SetWorldRotation` _springarm (`KismetMathLibrary.MakeRotator` _returnvalue_roll -35.0 _returnvalue_yaw) false false))

(event `self.Sphere.OnComponentEndOverlap`
  (params (OverlappedComponent :type "PrimitiveComponent Object Reference") (OtherActor :type "Actor Object Reference") (OtherComp :type "PrimitiveComponent Object Reference") (OtherBodyIndex :type Integer))
  (bind _asbp_bomb_bomb_character_2 (cast `/Game/BombBombLand/ThirdPerson/Blueprints/BP_BombBombCharacter2` OtherActor))
  (`PlayerController.SetViewTargetWithBlend` (`GameplayStatics.GetPlayerController` 0) _asbp_bomb_bomb_character_2 2.0 "VTBlend_Linear" 0.0 false))

(fn `UserConstructionScript`)