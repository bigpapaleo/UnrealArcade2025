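; Goal crystal that spins and floats in the level and triggers the win when its box is overlapped.
; Tick rotates the mesh and keeps calling Play on a timeline that applies a vertical world offset to the actor.
; Any overlap, with no actor check, prints "Won!" and plays a second timeline that lerps the mesh between hard-coded relative positions while forcing the cached player character to a fixed rotation.
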(event `self.ReceiveBeginPlay`
  (bind _asbp_bomb_bomb_character (cast `/Game/BombBombLand/ThirdPerson/Blueprints/BP_BombBombCharacter` (`GameplayStatics.GetPlayerCharacter` 0)))
  (set `self.As BP Third Person Character 1` _asbp_bomb_bomb_character))

(event `self.ReceiveTick`
  (params (DeltaSeconds :type "Float (single-precision)"))
  (`SceneComponent.K2_AddLocalRotation` (`self.StaticMeshComponent`) (struct :`Yaw` 0.3) false false)
  (bind (_direction _newtrack_0) (`Timeline|Timeline_0`)
    (:`Update`
      (`self.K2_AddActorWorldOffset` self (`KismetMathLibrary.MakeVector` 0.0 0.0 _newtrack_0) false false))))

(event `self.Box.OnComponentBeginOverlap`
  (params (OverlappedComponent :type "PrimitiveComponent Object Reference") (OtherActor :type "Actor Object Reference") (OtherComp :type "PrimitiveComponent Object Reference") (OtherBodyIndex :type Integer) (bFromSweep :type Boolean) (SweepResult :type "HitResult Structure (by ref)"))
  (`KismetSystemLibrary.PrintString` "Won!")
  (bind (_direction _newtrack_1) (`Timeline|Timeline`)
    (:`Update`
      (`SceneComponent.K2_SetRelativeLocation` (`self.StaticMeshComponent`) (`KismetMathLibrary.VLerp` (4300.0 -450.0 700.0) (4300.0 -450.0 850.0) _newtrack_1) false false)
      (`self.K2_SetActorRotation` (`self.As BP Third Person Character 1`) (struct :`Yaw` 180.0) false))))

(fn `UserConstructionScript`)