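; Player controller for the main menu that shows the menu widget and moves on to map selection.
; BeginPlay creates the menu, fades out the transition screen and adds the arcade input mapping context.
; The first key press fades in a transition widget and, after a delay, opens the map selection level.
; Root widget events keep game-only input without cursor; save-game and bot/two-player character-selection logic is left unconnected.
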(event `self.ReceiveBeginPlay`
  (`|ExecutionSequence`
    (:`then_0`
      (`self.Create_MainMenu_WB`)
      (`/Game/Blueprint/FunctionLibrary/FunctionLibrary.FadeOutTransitionScreen`)
      (bind _asmenu_game_mode (cast `/Game/Blueprint/Menu/MenuGameMode` (`GameplayStatics.GetGameMode`)))
      (set `self.As Menu Game Mode` _asmenu_game_mode))
    (:`then_1`
      (`KismetSystemLibrary.RetriggerableDelay` 30.0))
    (:`then_2`
      (`EnhancedInputSubsystemInterface.AddMappingContext` (pcsubsystem `EnhancedInputLocalPlayerSubsystem` (`GameplayStatics.GetPlayerController` 0)) "/Game/Blueprint/Input/ArcadeActionMapping.ArcadeActionMapping" 0 (struct)))))

(event `Key|AnyKey`
  (params (Key :type "Key Structure"))
  ; Sorry being rude and changing this on you
  (:`Pressed`
    (`/Engine/EditorBlueprintResources/StandardMacros.DoOnce` false
      (:`Completed`
        (bind _returnvalue (`|CreateWidget` "/Game/UI/LoadingScreens/WB_Transistion_Fades.WB_Transistion_Fades_C"))
        (`UserWidget.AddToViewport` _returnvalue 8)
        (`/Game/UI/LoadingScreens/WB_Transistion_Fades.Fade_In` _returnvalue)
        (`KismetSystemLibrary.Delay` 1.0)
        (`GameplayStatics.OpenLevelBySoftObjectPtr` "/Game/Maps/Lvl_MapSelection.Lvl_MapSelection")))))

(event `EnhancedInput|/Game/Blueprint/Input/IA_StartButton`
  (params (ActionValue :type Boolean) (ElapsedSeconds :type "Float (double-precision)") (TriggeredSeconds :type "Float (double-precision)") (InputAction :type "InputAction Object Reference" :default "/Game/Blueprint/Input/IA_StartButton.IA_StartButton"))
  (:`Started`
    (`KismetSystemLibrary.PrintString` "0000000")))

(event `self.OnRootWidgetAdded`
  (set `self.bShowMouseCursor` false :!label _label)
  (`WidgetBlueprintLibrary.SetInputMode_GameOnly` self))

(event `self.OnRootWidgetRemoved`
  (goto _label))

(fn `Create_MainMenu_WB`
  (bind _mainmenu_wb (`self.MainMenu_WB`)
    (:`then`
      (if (not (`Widget.IsInViewport` _mainmenu_wb))
        (`UserWidget.AddToViewport` _mainmenu_wb 0 :!label _label)))
    (:`else`
      (bind _returnvalue (`|CreateWidget` "/Game/UI/MainMenu/WB_MainMenu.WB_MainMenu_C" (`GameplayStatics.GetPlayerController` 0)))
      (set `self.MainMenu_WB` _returnvalue)
      (goto _label))))

(fn `UserConstructionScript`)