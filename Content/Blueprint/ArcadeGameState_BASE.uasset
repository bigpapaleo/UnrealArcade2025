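; Base arcade game state that keeps the current scores for a two-player match.
; PlayerHasDied takes the player who died and adds one point to the other player's score.
; Tick feeds a one-second Delay, so both scores print as debug strings about once per second.
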(event `self.ReceiveTick`
  (params (DeltaSeconds :type "Float (single-precision)"))
  (`KismetSystemLibrary.Delay` 1.0)
  (`KismetSystemLibrary.PrintString` (`KismetStringLibrary.Concat_StrStr` "Player 1 score -    " (`KismetStringLibrary.Conv_IntToString` (`self.Player1CurrentScore`))))
  (`KismetSystemLibrary.PrintString` (`KismetStringLibrary.Concat_StrStr` "Player 2 score -    " (`KismetStringLibrary.Conv_IntToString` (`self.Player2CurrentScore`)))))

(fn `PlayerHasDied`
  (params (PlayerNumbers :type "/Game/Blueprint/PlayerNumbers Enum" :default "NewEnumerator0"))
  (switch `/Game/Blueprint/PlayerNumbers` PlayerNumbers
    (:`NewEnumerator0`
      (set `self.Player2CurrentScore` (+ (`self.Player2CurrentScore`) 1)))
    (:`NewEnumerator1`
      (set `self.Player1CurrentScore` (+ (`self.Player1CurrentScore`) 1)))))

(fn `UserConstructionScript`)