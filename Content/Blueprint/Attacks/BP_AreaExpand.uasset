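; Expanding area attack actor that grows a mesh outward horizontally from spawn and notifies the player when it enters or leaves the circle.
; A Timeline starts on BeginPlay and lerps the mesh's X and Y scale at constant height, with a Delay on its update destroying the actor shortly after.
; Cylinder overlap events message the player character, using an IsOverlapping flag cleared one tick after exit to suppress repeated enter notifications.
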(event `self.ReceiveBeginPlay`
  (bind (_direction _newtrack_0) (`Timeline|Timeline`)
    (:`Update`
      (`SceneComponent.SetRelativeScale3D` (`self.StaticMesh`) (`KismetMathLibrary.VLerp` (1.0 1.0 5.0) (20.0 20.0 5.0) _newtrack_0))
      (`KismetSystemLibrary.Delay` 2.1)
      (`self.K2_DestroyActor`))))

(event `self.Cylinder.OnComponentBeginOverlap`
  (params (OverlappedComponent :type "PrimitiveComponent Object Reference") (OtherActor :type "Actor Object Reference") (OtherComp :type "PrimitiveComponent Object Reference") (OtherBodyIndex :type Integer) (bFromSweep :type Boolean) (SweepResult :type "HitResult Structure (by ref)"))
  (if (== OtherActor (`GameplayStatics.GetPlayerCharacter` 0))
    (if (not (`self.IsOverlapping`))
      (set `self.IsOverlapping` true)
      (message `/Game/Blueprint/Attacks/BPI_Attacks.IsOverlap_Circle` (`GameplayStatics.GetPlayerCharacter` 0)))))

(event `self.Cylinder.OnComponentEndOverlap`
  (params (OverlappedComponent :type "PrimitiveComponent Object Reference") (OtherActor :type "Actor Object Reference") (OtherComp :type "PrimitiveComponent Object Reference") (OtherBodyIndex :type Integer))
  (if (== OtherActor (`GameplayStatics.GetPlayerCharacter` 0))
    (message `/Game/Blueprint/Attacks/BPI_Attacks.NotOverlap_Circle` (`GameplayStatics.GetPlayerCharacter` 0))
    (`KismetSystemLibrary.DelayUntilNextTick`)
    (set `self.IsOverlapping` false)))

(fn `UserConstructionScript`)