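; Base game mode for a two-player local arcade shooter, running a match from spawn to end-of-round scoring.
; BeginPlay scatters walls inside spawner boxes, spawns and possesses both players at random starts, then sets up HUD and music.
; Looping one-second timers drive the input-locked intro countdown and the round clock, which ends by freezing players and showing kills.
; A retriggerable delay on any key starts an idle countdown that opens the credits map.
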(event `self.ReceiveBeginPlay`
  (`|ExecutionSequence`
    (:`then_0`
      (`self.SetUpPlayerStarts`)
      (`self.SetUpWalls`)
      (`self.EndLocalPlayer`)
      (`self.SpawnPlayers` false))
    (:`then_1`
      (`self.SetUpGameState`))
    (:`then_4`
      (bind _returnvalue (`|CreateWidget` "/Game/UI/Timer_UI.Timer_UI_C"))
      (set `self.Timer_UI` _returnvalue))
    (:`then_5`
      (`self.SetUpUI`))
    (:`then_7`
      (`self.GamePlayMusic`))
    (:`then_8`
      (`KismetSystemLibrary.Delay` 5.0)
      ; Game starts here
      (`self.IntroCoutntdown`))))

(event `NoInputChecker`
  ; No Input checking
  (bind _returnvalue (`KismetSystemLibrary.K2_SetTimerDelegate` (delegate `CheckForInput`) 1.0 true))
  (`/Engine/EditorBlueprintResources/StandardMacros.DoOnce` false
    (:`Completed`
      (`UserWidget.AddToViewport` (`self.Timer_UI`) 0))))

(event `Key|AnyKey`
  (params (Key :type "Key Structure"))
  ; No Input checking
  (:`Pressed`
    (`KismetSystemLibrary.RetriggerableDelay` 30.0)
    (`self.NoInputChecker`)))

(event `CheckForInput`
  (bind _backgroundtimerdispaly (`self.BackGroundTimerDispaly`))
  ; No Input checking
  (`/Game/UI/Timer_UI.CountdownTimer` (`self.Timer_UI`) _backgroundtimerdispaly)
  (bind _result (`/Engine/EditorBlueprintResources/StandardMacros.DecrementInt` _backgroundtimerdispaly)
    (:`  `
      (if (<= _result -1)
        (`KismetSystemLibrary.K2_ClearAndInvalidateTimerHandle` (stale `NoInputChecker` _returnvalue))
        (`GameplayStatics.OpenLevelBySoftObjectPtr` "/Game/Maps/CreditsMap.CreditsMap")))))

(event `IntroCoutntdown`
  (bind _returnvalue (`KismetSystemLibrary.K2_SetTimerDelegate` (delegate `IntroTimer`) 1.0 true))
  (bind _outactors (`GameplayStatics.GetAllActorsOfClass` "/Game/Blueprint/ArcadePlayerController_BASE.ArcadePlayerController_BASE_C"))
  (for _array_element _outactors
    (`/Game/Blueprint/ArcadePlayerController_BASE.DisableInputForIntro` _array_element)))

(event `IntroTimer`
  (bind _result (`/Engine/EditorBlueprintResources/StandardMacros.DecrementInt` (`self.IntroCountdown`))
    (:`  `
      (if (<= _result -1)
        (`KismetSystemLibrary.K2_ClearAndInvalidateTimerHandle` (stale `IntroCoutntdown` _returnvalue))
        (bind _hud (`self.HUD`)
          (:`then`
            (`/Game/UI/LevelheadTest.ClearTimer` _hud)
            (`self.GameplayCountdown`)
            (bind _outactors (`GameplayStatics.GetAllActorsOfClass` "/Game/Blueprint/ArcadePlayerController_BASE.ArcadePlayerController_BASE_C"))
            (for _array_element _outactors
              (`/Game/Blueprint/ArcadePlayerController_BASE.EnableInputForIntro` _array_element)
              (`self.SetUpCamera`)
              (`self.StartAmmoTimers`)))
          (:`else`))))))

(event `GameplayCountdown`
  (bind _returnvalue (`KismetSystemLibrary.K2_SetTimerDelegate` (delegate `GamePlayTimer`) 1.0 true))
  (`/Engine/EditorBlueprintResources/StandardMacros.DoOnce` false
    (:`Completed`
      (`/Game/UI/LevelheadTest.ShowHUDinfo` (`self.HUD`)))))

(event `GamePlayTimer`
  (bind _result (`/Engine/EditorBlueprintResources/StandardMacros.DecrementInt` (`self.GameTime`))
    (:`  `
      (if (<= _result 0)
        (`KismetSystemLibrary.K2_ClearAndInvalidateTimerHandle` (stale `GameplayCountdown` _returnvalue))
        (`self.EndOfround`)))))

(event `EndOfRound`
  (bind _as_arcade_game_state_base (`self.As Arcade Game State BASE`))
  (`WidgetLayoutLibrary.RemoveAllWidgets`)
  (bind _returnvalue (`|CreateWidget` "/Game/UI/EndOfRoundScoring_UI.EndOfRoundScoring_UI_C" null (`/Game/Blueprint/ArcadeGameState_BASE.Player1CurrentScore` _as_arcade_game_state_base) (`/Game/Blueprint/ArcadeGameState_BASE.Player2CurrentScore` _as_arcade_game_state_base)))
  (`UserWidget.AddToPlayerScreen` _returnvalue 0)
  (`/Game/UI/EndOfRoundScoring_UI.Set kills` _returnvalue)
  (bind _outactors (`GameplayStatics.GetAllActorsOfClass` "/Game/Blueprint/Player_BASE.Player_BASE_C"))
  (for _array_element _outactors
    (`/Game/Blueprint/Player_BASE.StopTimer` _array_element)
    (set `/Game/Blueprint/Player_BASE.CanShootWeaponOne?` false _array_element)
    (`CharacterMovementComponent.DisableMovement` (`Character.CharacterMovement` _array_element))))

(event `EndLocalPlayer`
  (`GameplayStatics.RemovePlayer` (`GameplayStatics.GetPlayerController` 1) true))

(fn `GamePlayMusic`
  (`GameplayStatics.PlaySound2D` "/Game/Assets/Audio/LevelGameplay.LevelGameplay" 1.0 1.0 0.0 null null))

(fn `RespawnPlayer`
  (params (PlayerNumbers :type "/Game/Blueprint/PlayerNumbers Enum" :default "NewEnumerator0"))
  (switch `/Game/Blueprint/PlayerNumbers` PlayerNumbers
    (:`NewEnumerator0`
      (`self.K2_TeleportTo` :`self` (`self.Player1Actor`) :`DestLocation` (`self.K2_GetActorLocation` (`KismetArrayLibrary.Array_Random` (`self.PlayerStartArray`)))))
    (:`NewEnumerator1`
      (`self.K2_TeleportTo` :`self` (`self.Player2Actor`) :`DestLocation` (`self.K2_GetActorLocation` (`KismetArrayLibrary.Array_Random` (`self.PlayerStartArray`)))))))

(fn `SetUpCamera`
  (bind _outactors (`GameplayStatics.GetAllActorsOfClass` "/Script/CinematicCamera.CineCameraActor"))
  (for _array_element _outactors
    (bind _outactors_2 (`GameplayStatics.GetAllActorsOfClass` "/Game/Blueprint/Player_BASE.Player_BASE_C"))
    (for (_ _array_index) _outactors_2
      (`PlayerController.SetViewTargetWithBlend` (`GameplayStatics.GetPlayerController` _array_index) _array_element 0.0 "VTBlend_Linear" 0.0 false))))

(fn `SetUpGameState`
  (bind _asarcade_game_state_base (cast `/Game/Blueprint/ArcadeGameState_BASE` (`GameplayStatics.GetGameState`)))
  (set `self.As Arcade Game State BASE` _asarcade_game_state_base))

(fn `SetUpPlayerStarts`
  (bind _outactors (`GameplayStatics.GetAllActorsOfClass` "/Script/Engine.PlayerStart"))
  (set `self.PlayerStartArray` _outactors))

(fn `SetUpUI`
  (bind _returnvalue (`|CreateWidget` "/Game/UI/LevelheadTest.LevelheadTest_C"))
  (bind _output_get (set `self.HUD` _returnvalue))
  (`UserWidget.AddToPlayerScreen` _output_get 0))

(fn `SetUpWalls`
  (bind _outactors (`GameplayStatics.GetAllActorsOfClass` "/Game/Blueprint/WallSpawner.WallSpawner_C"))
  (for _array_element _outactors
    (for _ (range 11)
      (bind _box (`/Game/Blueprint/WallSpawner.Box` _array_element))
      (`|SpawnActorFromClass` "/Game/Blueprint/Walls.Walls_C" (`KismetMathLibrary.MakeTransform` (`KismetMathLibrary.RandomPointInBoundingBox` (`SceneComponent.K2_GetComponentLocation` _box) (`BoxComponent.GetScaledBoxExtent` _box))) "Undefined" "MultiplyWithRoot" null null))))

(fn `SpawnPlayers`
  (params (`DoesItNeedBot?` :type Boolean))
  (bind _returnvalue (`GameplayStatics.GetPlayerController` 0))
  (bind _returnvalue_2 (`GameplayStatics.GetPlayerController` 1))
  (bind _outitem (`KismetArrayLibrary.Array_Random` (`self.PlayerStartArray`)))
  (if `DoesItNeedBot?`
    _
    (else
      _))
  (for _index (range (+ (`self.PlayerCount`) 1))
    (switch `int` _index
      (:`0`
        (`/Engine/EditorBlueprintResources/StandardMacros.DoOnce` false
          (:`Completed`
            (if (== (`self.Player1`) 0)
              (`GameplayStatics.CreatePlayer` 0)
              (bind _returnvalue_3 (`|SpawnActorFromClass` "/Game/Blueprint/Player_1.Player_1_C" (`self.GetTransform` _outitem) "Undefined" "MultiplyWithRoot" null 0 "NewEnumerator0" null))
              (set `self.Player1Actor` _returnvalue_3)
              (`Controller.Possess` _returnvalue _returnvalue_3)
              (set `PlayerController.bShowMouseCursor` false _returnvalue)))))
      (:`1`
        (`/Engine/EditorBlueprintResources/StandardMacros.DoOnce` false
          (:`Completed`
            (if (== (`self.Player2`) 1)
              (`GameplayStatics.CreatePlayer` 1)
              (bind _returnvalue_4 (`|SpawnActorFromClass` "/Game/Blueprint/Player_2.Player_2_C" (`self.GetTransform` _outitem) "Undefined" "MultiplyWithRoot" null 1 "NewEnumerator1" null))
              (set `self.Player2Actor` _returnvalue_4)
              (`Controller.Possess` _returnvalue_2 _returnvalue_4)
              (set `PlayerController.bShowMouseCursor` false _returnvalue_2))))))))

(fn `StartAmmoTimers`
  (bind _outactors (`GameplayStatics.GetAllActorsOfClass` "/Game/Blueprint/Player_BASE.Player_BASE_C"))
  (for _array_element _outactors
    (`/Game/Blueprint/Player_BASE.FillAmmoAtStart` _array_element)))

(fn `UserConstructionScript`)