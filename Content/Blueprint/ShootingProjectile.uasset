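; A projectile actor that destroys itself when it hits a wall or an opposing player.
; On BeginPlay its Collision component ignores ActorToIgnore while moving.
; On overlap it skips players whose number matches its own PlayerNumber; for others it calls KilledOtherPlayer on the player hit, behind a DoOnce that is reset right after, then destroys itself.
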(event `self.ReceiveBeginPlay`
  (`PrimitiveComponent.IgnoreActorWhenMoving` (`self.Collision`) (`self.ActorToIgnore`) true))

(event `self.Collision.OnComponentBeginOverlap`
  (params (OverlappedComponent :type "PrimitiveComponent Object Reference") (OtherActor :type "Actor Object Reference") (OtherComp :type "PrimitiveComponent Object Reference") (OtherBodyIndex :type Integer) (bFromSweep :type Boolean) (SweepResult :type "HitResult Structure (by ref)"))
  (cast `/Game/Blueprint/Walls` OtherActor
    (:`then`
      (`self.K2_DestroyActor` :!label _label))
    (:`CastFailed`
      (bind _asplayer_base (cast `/Game/Blueprint/Player_BASE` OtherActor))
      (if (not (`|EnumEquality` (`/Game/Blueprint/Player_BASE.PlayerNumbers` _asplayer_base) (`self.PlayerNumber`)))
        (`/Engine/EditorBlueprintResources/StandardMacros.DoOnce` false :!label _label_2
          (:`Completed`
            (`/Game/Blueprint/Player_BASE.KilledOtherPlayer` _asplayer_base)
            (`self.ResetKillPlayer`)
            (goto _label)))))))

(event `ResetKillPlayer`
  (goto _label_2 :!via `Reset`))

(fn `UserConstructionScript`)