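; Base player controller for the arcade mode that can lock and unlock the player character around an intro.
; DisableInputForIntro casts the controlled pawn to Player_BASE, sets its movement mode to None and clears CanShoot.
; EnableInputForIntro reverses this with Walking movement and shooting re-enabled.
; Both act on character state rather than the input system, and the file itself never calls them.
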(fn `DisableInputForIntro`
  (bind _asplayer_base (cast `/Game/Blueprint/Player_BASE` (`self.K2_GetPawn`)))
  (`CharacterMovementComponent.SetMovementMode` (`Character.CharacterMovement` _asplayer_base) "MOVE_None" 0)
  (set `/Game/Blueprint/Player_BASE.CanShoot?` false _asplayer_base))

(fn `EnableInputForIntro`
  (bind _asplayer_base (cast `/Game/Blueprint/Player_BASE` (`self.K2_GetPawn`)))
  (`CharacterMovementComponent.SetMovementMode` (`Character.CharacterMovement` _asplayer_base) "MOVE_Walking" 0)
  (set `/Game/Blueprint/Player_BASE.CanShoot?` true _asplayer_base))

(fn `UserConstructionScript`)