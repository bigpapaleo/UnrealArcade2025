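; Game mode for a two-player menu test that sets up two local players sharing one widget.
; On BeginPlay it creates players for controllers 0 and 1, then adds a TwoControllersTestWidget to the player screen.
; Each player is set as owning player of its own input sub-widget within that widget.
; A disconnected branch that would remove and destroy existing player controllers before setup never runs.
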(event `self.ReceiveBeginPlay`
  (bind _returnvalue (`GameplayStatics.CreatePlayer` 0))
  (bind _output_get (set `self.Player1` _returnvalue))
  (bind _returnvalue_2 (`GameplayStatics.CreatePlayer` 1))
  (bind _output_get_2 (set `self.Player2` _returnvalue_2))
  (bind _returnvalue_3 (`|CreateWidget` "/Game/UI/TwoControllersTestWidget.TwoControllersTestWidget_C"))
  (`UserWidget.AddToPlayerScreen` _returnvalue_3 0)
  (`UserWidget.SetOwningPlayer` (`/Game/UI/TwoControllersTestWidget.PlayerOneInput` _returnvalue_3) _output_get)
  (`UserWidget.SetOwningPlayer` (`/Game/UI/TwoControllersTestWidget.PlayerTwoInput` _returnvalue_3) _output_get_2))

(fn `UserConstructionScript`)