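; Actor that endlessly spins a skeletal mesh and swaps it at random between five characters and models, with a poof effect on each swap.
; A timeline drives the yaw, then on finish picks a new mesh and restarts itself.
; ChooseNewMesh rolls the mesh and passes it to the SameAsLast macro, which is meant to re-roll repeats and otherwise applies the mesh and a transform.
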(event `self.ReceiveBeginPlay`
  (`self.Rotate/Switch_Cube`)
  (`self.ChooseNewMesh`))

(event `Rotate/Switch_Cube`
  (bind (_direction _newtrack_0) (`Timeline|Timeline` :!via `PlayFromStart`)
    (:`Update`
      (`SceneComponent.K2_SetRelativeRotation` (`self.SkeletalMesh`) (`KismetMathLibrary.MakeRotator` 0.0 0.0 _newtrack_0) false false))
    (:`Finished`
      (`self.ChooseNewMesh`)
      (`self.Rotate/Switch_Cube`))))

(fn `ChooseNewMesh`
  ;[0.1979 0.1979 0.1979] Randomly selects a new mesh and sets it
  (switch `int` (`KismetMathLibrary.RandomIntegerInRange` 0 4)
    (:`0`
      (`self.SameAsLast?` "/Game/REHorror/Models/Character/NaomiWoulfe/SK_NaomiWoulf.SK_NaomiWoulf"
        (:`New`
          _)))
    (:`1`
      (`self.SameAsLast?` "/Game/Assets/Characters/WindClan/SK_WindClan_Test.SK_WindClan_Test"
        (:`New`
          _)))
    (:`2`
      (`self.SameAsLast?` "/Game/Adrian/SKM_Battie.SKM_Battie"
        (:`New`
          _)))
    (:`3`
      (`self.SameAsLast?` "/Game/Assets/Characters/Spaceship/SKM_ArcadeCabinetShip1.SKM_ArcadeCabinetShip1"
        (:`New`
          _)))
    (:`4`
      (`self.SameAsLast?` "/Game/BombBombLand/LearningKit_Games/Assets/Characters/Character/Mesh/SK_EpicCharacter.SK_EpicCharacter"
        (:`New`
          _))))
  (`NiagaraFunctionLibrary.SpawnSystemAtLocation` "/Game/MythOfLegndrule/Effects/P_Poof.P_Poof" (`SceneComponent.K2_GetComponentLocation` (`self.SkeletalMesh`)) (struct) (3.0 3.0 3.0))
  (return))

(fn `UserConstructionScript`)